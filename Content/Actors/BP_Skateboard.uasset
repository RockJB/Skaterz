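; Skateboard actor that tilts its pitch to follow the slope of the ground, or eases to a fixed nose-up angle while jumping.
; A short downward trace from the Sphere, with debug drawing, gets the surface normal.
; Cross products project the forward vector onto that surface, and its Z is mapped to a clamped pitch.
; Tick lerps toward that pitch by delta time and interp speed, preserving yaw and roll.
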(event `self.ReceiveTick`
  (params (DeltaSeconds :type "Float (single-precision)"))
  (bind _returnvalue (`SceneComponent.K2_GetComponentLocation` (`self.Sphere`)))
  (if (`self.IsJumping`)
    (`self.Lerp To Desired Pitch` 15.0 DeltaSeconds)
    (else
      (bind _outhit (`KismetSystemLibrary.LineTraceSingle` :`Start` (+ _returnvalue (0.0 0.0 20.0)) :`End` (+ _returnvalue (0.0 0.0 -100.0)) :`TraceChannel` "TraceTypeQuery1" :`DrawDebugType` "ForOneFrame"))
      (bind (_bblockinghit _binitialoverlap _time _distance _location _impactpoint _normal) (`GameplayStatics.BreakHitResult` _outhit))
      (set `self.DesiredPitch` (`KismetMathLibrary.MapRangeClamped` (.z (`KismetMathLibrary.Normal` (`KismetMathLibrary.Cross_VectorVector` _normal (`KismetMathLibrary.Normal` (`KismetMathLibrary.Cross_VectorVector` (`self.GetActorForwardVector`) _normal))))) -1.0 1.0 -45.0 45.0))
      (`self.Lerp To Desired Pitch` (`self.DesiredPitch`) DeltaSeconds))))

(fn `Lerp To Desired Pitch`
  (params (`Desired Pitch` :type "Float (double-precision)") (`Delta Seconds` :type "Float (double-precision)"))
  (bind (_returnvalue_roll _returnvalue_pitch) (`KismetMathLibrary.BreakRotator` (`self.K2_GetActorRotation`)))
  (bind (_returnvalue_roll_2 _returnvalue_pitch_2 _returnvalue_yaw) (`KismetMathLibrary.BreakRotator` (`self.K2_GetActorRotation`)))
  (set `self.CurrentPitch` _returnvalue_pitch)
  (set `self.NextPitch` (`KismetMathLibrary.Lerp` (`self.CurrentPitch`) `Desired Pitch` (* `Delta Seconds` (`self.PitchInterpSpeed`))))
  (`self.K2_SetActorRotation` (`KismetMathLibrary.MakeRotator` _returnvalue_roll_2 (`self.NextPitch`) _returnvalue_yaw)))

(fn `UserConstructionScript`
  (set `self.Board` (`self.SkateBoard_Plane_005`)))