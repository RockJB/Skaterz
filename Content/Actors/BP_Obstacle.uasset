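; BP_Obstacle is an obstacle actor that awards points when the player character passes out of its points collider.
; On BeginPlay it writes PointsAwardedVal into two UI_WorldPoints widgets, Widget and WidgetMirror, to display its value.
; When BP_ThirdPersonCharacter ends overlap with ColliderPoints, it adds that value to the game mode's Points and calls CallOnPointsChanged.
; The begin-overlap handler only casts and has no effect.
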(event `self.ReceiveBeginPlay`
  (bind _asui_world_points (cast `/Game/UI/UI_WorldPoints` (`WidgetComponent.GetWidget` (`self.Widget`))))
  (`/Game/UI/UI_WorldPoints.SetPointsValue` _asui_world_points (`self.PointsAwardedVal`))
  (bind _asui_world_points_2 (cast `/Game/UI/UI_WorldPoints` (`WidgetComponent.GetWidget` (`self.WidgetMirror`))))
  (`/Game/UI/UI_WorldPoints.SetPointsValue` _asui_world_points_2 (`self.PointsAwardedVal`)))

(event `self.ColliderPoints.OnComponentBeginOverlap`
  (params (OverlappedComponent :type "PrimitiveComponent Object Reference") (OtherActor :type "Actor Object Reference") (OtherComp :type "PrimitiveComponent Object Reference") (OtherBodyIndex :type Integer) (bFromSweep :type Boolean) (SweepResult :type "HitResult Structure (by ref)"))
  (cast `/Game/ThirdPerson/Blueprints/BP_ThirdPersonCharacter` OtherActor))

(event `self.ColliderPoints.OnComponentEndOverlap`
  (params (OverlappedComponent :type "PrimitiveComponent Object Reference") (OtherActor :type "Actor Object Reference") (OtherComp :type "PrimitiveComponent Object Reference") (OtherBodyIndex :type Integer))
  (cast `/Game/ThirdPerson/Blueprints/BP_ThirdPersonCharacter` OtherActor)
  (bind _asbp_third_person_game_mode (cast `/Game/ThirdPerson/Blueprints/BP_ThirdPersonGameMode` (`GameplayStatics.GetGameMode`)))
  (set `/Game/ThirdPerson/Blueprints/BP_ThirdPersonGameMode.Points` (+ (`/Game/ThirdPerson/Blueprints/BP_ThirdPersonGameMode.Points` _asbp_third_person_game_mode) (`self.PointsAwardedVal`)) _asbp_third_person_game_mode)
  (`/Game/ThirdPerson/Blueprints/BP_ThirdPersonGameMode.OnPointsChanged` _asbp_third_person_game_mode))

(fn `UserConstructionScript`)